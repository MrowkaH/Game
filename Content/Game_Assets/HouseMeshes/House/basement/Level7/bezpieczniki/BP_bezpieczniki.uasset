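; Fuse box in the house basement that the player opens, then switches to send a turn-on message to a linked actor.
; Overlapping the collision enables input and shows one of two prompt widgets, depending on whether the door is open.
; The first interact swings the door open with a timeline.
; Once open, interacting rotates the Flicker switch on a second timeline, which calls CanTurnOnMessage on the linked actor when finished.
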(event `self.ReceiveBeginPlay`
  (bind _asbp_first_person_character (cast `/Game/FirstPerson/Blueprints/BP_FirstPersonCharacter` (`GameplayStatics.GetPlayerCharacter` 0)))
  (set `self.As BP First Person Character` _asbp_first_person_character))

(event `self.coll.OnComponentBeginOverlap`
  (params (OverlappedComponent :type "PrimitiveComponent Object Reference") (OtherActor :type "Actor Object Reference") (OtherComp :type "PrimitiveComponent Object Reference") (OtherBodyIndex :type Integer) (bFromSweep :type Boolean) (SweepResult :type "HitResult Structure (by ref)"))
  (bind _returnvalue (`GameplayStatics.GetPlayerController` 0))
  (if (== OtherActor (`self.As BP First Person Character`))
    (if (`self.DidOpen?`)
      (`SceneComponent.SetVisibility` (`self.Widget1`) true false)
      (`self.EnableInput` _returnvalue)
      (else
        (`SceneComponent.SetVisibility` (`self.Widget`) true false)
        (`self.EnableInput` _returnvalue)))))

(event `self.coll.OnComponentEndOverlap`
  (params (OverlappedComponent :type "PrimitiveComponent Object Reference") (OtherActor :type "Actor Object Reference") (OtherComp :type "PrimitiveComponent Object Reference") (OtherBodyIndex :type Integer))
  (bind _returnvalue (`GameplayStatics.GetPlayerController` 0))
  (if (== (`self.As BP First Person Character`) OtherActor)
    (if (`self.DidOpen?`)
      (`SceneComponent.SetVisibility` (`self.Widget1`) false false)
      (`self.DisableInput` _returnvalue)
      (else
        (`SceneComponent.SetVisibility` (`self.Widget`) false false)
        (`self.DisableInput` _returnvalue)))))

(event `MoveDoors`
  (bind (_direction _move) (`Timeline|open`)
    (:`Update`
      (`SceneComponent.K2_SetRelativeTransform` (`self.doors`) (`KismetMathLibrary.MakeTransform` (0.0 0.0 0.0) (`KismetMathLibrary.RLerp` (struct) (struct :`Yaw` 130.0) _move)) false false))
    (:`Finished`
      (set `self.DidOpen?` true)
      (`SceneComponent.SetVisibility` (`self.Widget`) false false)
      (`SceneComponent.SetVisibility` (`self.Widget1`) true false))))

(event `EnhancedInput|/Game/FirstPerson/Input/Actions/IA_Interact`
  (params (ActionValue :type Boolean) (ElapsedSeconds :type "Float (double-precision)") (TriggeredSeconds :type "Float (double-precision)") (InputAction :type "InputAction Object Reference" :default "/Game/FirstPerson/Input/Actions/IA_Interact.IA_Interact"))
  (:`Started`
    (if (`self.DidOpen?`)
      (`self.TurnOnLight`)
      (else
        (`self.MoveDoors`)))))

(event `TurnOnLight`
  (bind _returnvalue_location (`KismetMathLibrary.BreakTransform` (`SceneComponent.GetRelativeTransform` (`self.flicker`))))
  (bind (_direction _move) (`Timeline|Timeline`)
    (:`Update`
      (`SceneComponent.K2_SetRelativeTransform` (`self.flicker`) (`KismetMathLibrary.MakeTransform` _returnvalue_location (`KismetMathLibrary.RLerp` (struct :`Pitch` -90.0) (struct) _move)) false false))
    (:`Finished`
      (message `/Game/Game_Assets/Lightning/bps/BPI_Lighton.CanTurnOn` (`self.actor`)))))

(fn `UserConstructionScript`)