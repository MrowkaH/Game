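; BP_Piano is a piano actor that builds its keyboard at BeginPlay by spawning separate white and black key actors.
; A loop spawns white keys at even steps along world X from the actor's transform.
; Nested loops spawn black keys from the stored SpawnLocB transform, stepping along negative X with alternating short and long gaps.
; Offsets accumulate in vector variables and are added to location without being rotated by the actor's rotation.
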(event `self.ReceiveBeginPlay`
  (bind (_offset4key_x _offset4key_y _offset4key_z) (`KismetMathLibrary.BreakVector` (`self.Offset4Key`)))
  (bind (_offset4key_b_x _offset4key_b_y _offset4key_b_z) (`KismetMathLibrary.BreakVector` (`self.Offset4Key_B`)))
  (bind (_offset4key_b_x_2 _offset4key_b_y_2 _offset4key_b_z_2) (`KismetMathLibrary.BreakVector` (`self.Offset4Key_B`)))
  (for _ (range 1 34)
    (set `self.Offset4Key` (`KismetMathLibrary.MakeVector` (+ _offset4key_x 7.5) _offset4key_y _offset4key_z))
    (bind _output_get (set `self.SpawnLocW` (`self.GetTransform`)))
    (`|SpawnActorFromClass` (`self.KeyWhite`) (`KismetMathLibrary.MakeTransform` (+ (.location _output_get) (`self.Offset4Key`)) (.rotation _output_get) (.scale _output_get)) "AlwaysSpawn" "MultiplyWithRoot" null null))
  (for _ (range 2)
    (for _ (range 4)
      (set `self.Offset4Key_B` (`KismetMathLibrary.MakeVector` (+ _offset4key_b_x_2 -8.0) _offset4key_b_y_2 _offset4key_b_z_2))
      (bind _output_get_2 (set `self.SpawnLocB` (`self.SpawnLocB`)))
      (`|SpawnActorFromClass` (`self.KeyBlack`) (`KismetMathLibrary.MakeTransform` (+ (.location _output_get_2) (`self.Offset4Key_B`)) (.rotation _output_get_2) (.scale _output_get_2)) "AlwaysSpawn" "MultiplyWithRoot" null null)
      (for _ (range 1)
        (set `self.Offset4Key_B` (`KismetMathLibrary.MakeVector` (+ _offset4key_b_x -16.0) _offset4key_b_y _offset4key_b_z))
        (bind _output_get_3 (set `self.SpawnLocB` (`self.SpawnLocB`)))
        (`|SpawnActorFromClass` (`self.KeyBlack`) (`KismetMathLibrary.MakeTransform` (+ (.location _output_get_3) (`self.Offset4Key_B`)) (.rotation _output_get_3) (.scale _output_get_3)) "AlwaysSpawn" "MultiplyWithRoot" null null)))))

(fn `UserConstructionScript`)