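; Flickering light bulb that hides a key and can be unscrewed by the player.
; BeginPlay spawns the KeyInside actor on the bulb's ForKey socket and starts a self-recalling random-delay flicker.
; Overlapping Coll shows a prompt widget and lets IA_F start a Timeline that moves and rotates the bulb.
; When it finishes, the bulb is destroyed and a faster flicker runs until the light and trigger are removed.
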(event `self.ReceiveBeginPlay`
  (bind _returnvalue (`|SpawnActorFromClass` (`self.KeyInside`) (`KismetMathLibrary.Conv_VectorToTransform` (`SceneComponent.GetSocketLocation` (`self.Bulb`) "None")) "AlwaysSpawn" "MultiplyWithRoot" null null))
  (`self.K2_AttachToComponent` _returnvalue (`self.Bulb`) "ForKey" "SnapToTarget" "KeepRelative" "KeepRelative" true)
  (`self.K2_SetActorRelativeRotation` _returnvalue (struct :`Pitch` 90.0 :`Yaw` 60.0) false false)
  (`self.SetActorRelativeScale3D` _returnvalue (0.8 0.8 0.8))
  (if (not false)
    (`self.Flicker`)))

(event `Open`
  (bind _bulb (`self.Bulb`))
  (bind (_direction _rotation _height) (`Timeline|Timeline`)
    (:`Update`
      (`SceneComponent.K2_SetRelativeLocation` _bulb (`KismetMathLibrary.MakeVector` 0.0 0.0 _height) false false)
      (`SceneComponent.K2_SetRelativeRotation` _bulb (`KismetMathLibrary.MakeRotator` 0.0 0.0 _rotation) false false))
    (:`Finished`
      (`ActorComponent.K2_DestroyComponent` (`self.Bulb`))
      (`self.Flickerdead`)
      (`KismetSystemLibrary.Delay` 2.5)
      (`ActorComponent.K2_DestroyComponent` (`self.PointLight`))
      (`ActorComponent.K2_DestroyComponent` (`self.Coll`))
      (set `self.IsAlive?` false))))

(event `EnhancedInput|/Game/FirstPerson/Input/Actions/IA_F`
  (params (ActionValue :type Boolean) (ElapsedSeconds :type "Float (double-precision)") (TriggeredSeconds :type "Float (double-precision)") (InputAction :type "InputAction Object Reference" :default "/Game/FirstPerson/Input/Actions/IA_F.IA_F"))
  (:`Started`
    (if (`self.CanOpen?`)
      (`self.Open`))))

(event `self.Coll.OnComponentBeginOverlap`
  (params (OverlappedComponent :type "PrimitiveComponent Object Reference") (OtherActor :type "Actor Object Reference") (OtherComp :type "PrimitiveComponent Object Reference") (OtherBodyIndex :type Integer) (bFromSweep :type Boolean) (SweepResult :type "HitResult Structure (by ref)"))
  (cast `/Game/FirstPerson/Blueprints/BP_FirstPersonCharacter` OtherActor)
  (`SceneComponent.SetVisibility` (`self.Widget`) true false)
  (set `self.CanOpen?` true))

(event `self.Coll.OnComponentEndOverlap`
  (params (OverlappedComponent :type "PrimitiveComponent Object Reference") (OtherActor :type "Actor Object Reference") (OtherComp :type "PrimitiveComponent Object Reference") (OtherBodyIndex :type Integer))
  (cast `/Game/FirstPerson/Blueprints/BP_FirstPersonCharacter` OtherActor)
  (`SceneComponent.SetVisibility` (`self.Widget`) false false)
  (set `self.CanOpen?` false))

(event `Flickerdead`
  ; Flickers
  (if (`self.IsAlive?`)
    (`SceneComponent.ToggleVisibility` (`self.PointLight`) false)
    (`KismetSystemLibrary.Delay` (`KismetMathLibrary.RandomFloatInRange` 0.1 0.2))
    (`self.Flickerdead`)))

(event `Flicker`
  ; Flickers
  (if (`self.IsAlive?`)
    (`SceneComponent.ToggleVisibility` (`self.PointLight`) false)
    (`KismetSystemLibrary.Delay` (`KismetMathLibrary.RandomFloatInRange` 0.05 2.0))
    (`self.Flicker`)))

(fn `UserConstructionScript`)