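; Readable note actor for basement Level 6 that the player can pick up and inspect with the F key.
; An overlap volume shows a prompt widget component and enables input while the player is inside.
; F toggles between freezing movement and look while a timeline lerps the note to the character's Note anchor, and restoring control while reversing it.
; A second FlipFlop on timeline finish alternately creates and hides the BPW_Note6_2 screen widget.
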(event `self.ReceiveBeginPlay`
  (bind _note (`self.Note`))
  (bind _asbp_first_person_character (cast `/Game/FirstPerson/Blueprints/BP_FirstPersonCharacter` (`GameplayStatics.GetPlayerCharacter` 0)))
  (set `self.As BP First Person Character` _asbp_first_person_character)
  (`SceneComponent.K2_AttachToComponent` (`self.Widget`) (`self.Note`) "None" "SnapToTarget" "KeepRelative" "KeepRelative" true)
  (set `self.OriginLoc` (`SceneComponent.K2_GetComponentLocation` _note))
  (set `self.OriginRot` (`SceneComponent.K2_GetComponentRotation` _note)))

(event `self.coll.OnComponentBeginOverlap`
  (params (OverlappedComponent :type "PrimitiveComponent Object Reference") (OtherActor :type "Actor Object Reference") (OtherComp :type "PrimitiveComponent Object Reference") (OtherBodyIndex :type Integer) (bFromSweep :type Boolean) (SweepResult :type "HitResult Structure (by ref)"))
  (if (== OtherActor (`self.As BP First Person Character`))
    (`SceneComponent.SetVisibility` (`self.Widget`) true false)
    (`self.EnableInput` (`GameplayStatics.GetPlayerController` 0))))

(event `self.coll.OnComponentEndOverlap`
  (params (OverlappedComponent :type "PrimitiveComponent Object Reference") (OtherActor :type "Actor Object Reference") (OtherComp :type "PrimitiveComponent Object Reference") (OtherBodyIndex :type Integer))
  (if (== (`self.As BP First Person Character`) OtherActor)
    (`SceneComponent.SetVisibility` (`self.Widget`) false false)
    (`self.DisableInput` (`GameplayStatics.GetPlayerController` 0))))

(event `EnhancedInput|/Game/FirstPerson/Input/Actions/IA_F`
  (params (ActionValue :type Boolean) (ElapsedSeconds :type "Float (double-precision)") (TriggeredSeconds :type "Float (double-precision)") (InputAction :type "InputAction Object Reference" :default "/Game/FirstPerson/Input/Actions/IA_F.IA_F"))
  (bind _returnvalue (`PlayerState.GetPlayerController` (`Pawn.PlayerState` (`self.As BP First Person Character`))))
  (bind (_returnvalue_location _returnvalue_rotation) (`KismetMathLibrary.BreakTransform` (`SceneComponent.K2_GetComponentToWorld` (`/Game/FirstPerson/Blueprints/BP_FirstPersonCharacter.note` (`self.As BP First Person Character`)))))
  (:`Started`
    (`/Engine/EditorBlueprintResources/StandardMacros.FlipFlop`
      (:`A`
        (`CharacterMovementComponent.DisableMovement` (`Character.CharacterMovement` (`GameplayStatics.GetPlayerCharacter` 0)))
        (`Controller.SetIgnoreLookInput` _returnvalue true)
        (bind (_direction _newtrack_0) (`Timeline|Move` :!label _label)
          (:`Update`
            (`SceneComponent.K2_SetWorldTransform` (`self.Note`) (`KismetMathLibrary.MakeTransform` (`KismetMathLibrary.VLerp` (`self.OriginLoc`) _returnvalue_location _newtrack_0) (`KismetMathLibrary.RLerp` (`self.OriginRot`) _returnvalue_rotation _newtrack_0)) false false))
          (:`Finished`
            (`/Engine/EditorBlueprintResources/StandardMacros.FlipFlop`
              (:`A`
                (bind _returnvalue_2 (`|CreateWidget` "/Game/Game_Assets/HouseMeshes/House/basement/Level6/Notatka/BPW_Note6_2.BPW_Note6_2_C"))
                (`UserWidget.AddToViewport` _returnvalue_2 0)
                (`Widget.SetVisibility` _returnvalue_2 "Visible"))
              (:`B`
                (`Widget.SetVisibility` _returnvalue_2 "Hidden"))))))
      (:`B`
        (`CharacterMovementComponent.SetMovementMode` (`Character.CharacterMovement` (`GameplayStatics.GetPlayerCharacter` 0)) "MOVE_Walking" 0)
        (`Controller.ResetIgnoreLookInput` _returnvalue)
        (goto _label :!via `Reverse`)))))

(fn `UserConstructionScript`)