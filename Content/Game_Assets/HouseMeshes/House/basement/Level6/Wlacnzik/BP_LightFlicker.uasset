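; BP_LightFlicker is a player-operated switch that rotates a Button component between two positions; no light logic is present despite the name.
; Overlapping the Coll volume as the first-person character shows a prompt widget and enables input, and leaving reverses both.
; Pressing IA_F while in range calls Click, where a FlipFlop alternately plays and reverses the Move timeline that drives the button's pitch.
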(event `self.ReceiveBeginPlay`
  (bind _asbp_first_person_character (cast `/Game/FirstPerson/Blueprints/BP_FirstPersonCharacter` (`GameplayStatics.GetPlayerCharacter` 0)))
  (set `self.As BP First Person Character` _asbp_first_person_character))

(event `Click`
  (`/Engine/EditorBlueprintResources/StandardMacros.FlipFlop`
    (:`A`
      (bind (_direction _move) (`Timeline|Move` :!label _label)
        (:`Update`
          (`SceneComponent.K2_SetRelativeRotation` (`self.Button`) (`KismetMathLibrary.MakeRotator` 0.0 _move) false false))))
    (:`B`
      (goto _label :!via `Reverse`))))

(event `EnhancedInput|/Game/FirstPerson/Input/Actions/IA_F`
  (params (ActionValue :type Boolean) (ElapsedSeconds :type "Float (double-precision)") (TriggeredSeconds :type "Float (double-precision)") (InputAction :type "InputAction Object Reference" :default "/Game/FirstPerson/Input/Actions/IA_F.IA_F"))
  (:`Started`
    (`KismetSystemLibrary.PrintString` "pressed")
    (if (`self.CanClick?`)
      (`self.Click`))))

(event `self.coll.OnComponentBeginOverlap`
  (params (OverlappedComponent :type "PrimitiveComponent Object Reference") (OtherActor :type "Actor Object Reference") (OtherComp :type "PrimitiveComponent Object Reference") (OtherBodyIndex :type Integer) (bFromSweep :type Boolean) (SweepResult :type "HitResult Structure (by ref)"))
  (if (== OtherActor (`self.As BP First Person Character`))
    (`SceneComponent.SetVisibility` (`self.Widget`) true false)
    (set `self.CanClick?` true)
    (`self.EnableInput` (`GameplayStatics.GetPlayerController` 0))))

(event `self.coll.OnComponentEndOverlap`
  (params (OverlappedComponent :type "PrimitiveComponent Object Reference") (OtherActor :type "Actor Object Reference") (OtherComp :type "PrimitiveComponent Object Reference") (OtherBodyIndex :type Integer))
  (if (== OtherActor (`self.As BP First Person Character`))
    (`SceneComponent.SetVisibility` (`self.Widget`) false false)
    (set `self.CanClick?` false)
    (`self.DisableInput` (`GameplayStatics.GetPlayerController` 0))))

(fn `UserConstructionScript`)