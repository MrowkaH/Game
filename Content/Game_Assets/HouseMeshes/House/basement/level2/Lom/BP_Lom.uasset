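; BP_Lom is an item actor that shows a widget when the first-person player character is nearby.
; On BeginPlay it caches the player character and attaches the widget to the "widget" socket on the Lom component.
; Coll overlap begin and end show and hide the widget, skipped while the character's HeldItem is this actor.
; Pickup logic is not handled in this Blueprint's graphs.
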(event `self.ReceiveBeginPlay`
  (bind _asbp_first_person_character (cast `/Game/FirstPerson/Blueprints/BP_FirstPersonCharacter` (`GameplayStatics.GetPlayerCharacter` 0)))
  (set `self.As BP First Person Character` _asbp_first_person_character)
  (`SceneComponent.K2_AttachToComponent` (`self.Widget`) (`self.Lom`) "widget" "KeepRelative" "KeepRelative" "KeepRelative" true))

(event `self.coll.OnComponentBeginOverlap`
  (params (OverlappedComponent :type "PrimitiveComponent Object Reference") (OtherActor :type "Actor Object Reference") (OtherComp :type "PrimitiveComponent Object Reference") (OtherBodyIndex :type Integer) (bFromSweep :type Boolean) (SweepResult :type "HitResult Structure (by ref)"))
  (bind _as_bp_first_person_character (`self.As BP First Person Character`))
  (if (== OtherActor _as_bp_first_person_character)
    (if (not (== (`/Game/FirstPerson/Blueprints/BP_FirstPersonCharacter.HeldItem` _as_bp_first_person_character) self))
      (`SceneComponent.SetVisibility` (`self.Widget`) true false))))

(event `self.coll.OnComponentEndOverlap`
  (params (OverlappedComponent :type "PrimitiveComponent Object Reference") (OtherActor :type "Actor Object Reference") (OtherComp :type "PrimitiveComponent Object Reference") (OtherBodyIndex :type Integer))
  (bind _as_bp_first_person_character (`self.As BP First Person Character`))
  (if (== _as_bp_first_person_character OtherActor)
    (if (not (== (`/Game/FirstPerson/Blueprints/BP_FirstPersonCharacter.HeldItem` _as_bp_first_person_character) self))
      (`SceneComponent.SetVisibility` (`self.Widget`) false false))))

(fn `UserConstructionScript`)