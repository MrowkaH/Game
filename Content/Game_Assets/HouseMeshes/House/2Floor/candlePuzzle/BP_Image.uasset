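; Rotating-painting puzzle in the house where four paintings must match their target rotations to trigger a key move on a referenced painting.
; Overlap volumes select a painting, show its widget and glow, and enable interact input.
; Interacting plays a shared timeline that turns the painting 90 degrees and stores its rounded rotation.
; Each check calls TurnOffcandle for correct paintings and, when all match, marks the puzzle solved and calls AttachkeyMove.
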(event `self.ReceiveBeginPlay`
  (bind _asbp_first_person_character (cast `/Game/FirstPerson/Blueprints/BP_FirstPersonCharacter` (`GameplayStatics.GetPlayerCharacter` 0)))
  (set `self.As BP First Person Character` _asbp_first_person_character))

(event `self.coll1.OnComponentBeginOverlap`
  (params (OverlappedComponent :type "PrimitiveComponent Object Reference") (OtherActor :type "Actor Object Reference") (OtherComp :type "PrimitiveComponent Object Reference") (OtherBodyIndex :type Integer) (bFromSweep :type Boolean) (SweepResult :type "HitResult Structure (by ref)"))
  (if (== OtherActor (`self.As BP First Person Character`))
    (if (not (`self.Solved?`))
      (`SceneComponent.SetVisibility` (`self.Widget1`) true false)
      (`MeshComponent.SetScalarParameterValueOnMaterials` (`self.obraz1`) "Glow Int" 1.0)
      (set `self.Index` 0)
      (`self.EnableInput` (`GameplayStatics.GetPlayerController` 0)))))

(event `self.coll1.OnComponentEndOverlap`
  (params (OverlappedComponent :type "PrimitiveComponent Object Reference") (OtherActor :type "Actor Object Reference") (OtherComp :type "PrimitiveComponent Object Reference") (OtherBodyIndex :type Integer))
  (if (== (`self.As BP First Person Character`) OtherActor)
    (if (not (`self.Solved?`))
      (`SceneComponent.SetVisibility` (`self.Widget1`) false false)
      (`MeshComponent.SetScalarParameterValueOnMaterials` (`self.obraz1`) "Glow Int" 0.0)
      (set `self.Index` -1)
      (`self.DisableInput` (`GameplayStatics.GetPlayerController` 0)))))

(event `self.coll2.OnComponentBeginOverlap`
  (params (OverlappedComponent :type "PrimitiveComponent Object Reference") (OtherActor :type "Actor Object Reference") (OtherComp :type "PrimitiveComponent Object Reference") (OtherBodyIndex :type Integer) (bFromSweep :type Boolean) (SweepResult :type "HitResult Structure (by ref)"))
  (if (== OtherActor (`self.As BP First Person Character`))
    (if (not (`self.Solved?`))
      (`SceneComponent.SetVisibility` (`self.Widget2`) true false)
      (`MeshComponent.SetScalarParameterValueOnMaterials` (`self.obraz2`) "Glow Int" 1.0)
      (set `self.Index` 1)
      (`self.EnableInput` (`GameplayStatics.GetPlayerController` 0)))))

(event `self.coll2.OnComponentEndOverlap`
  (params (OverlappedComponent :type "PrimitiveComponent Object Reference") (OtherActor :type "Actor Object Reference") (OtherComp :type "PrimitiveComponent Object Reference") (OtherBodyIndex :type Integer))
  (if (== (`self.As BP First Person Character`) OtherActor)
    (if (not (`self.Solved?`))
      (`SceneComponent.SetVisibility` (`self.Widget2`) false false)
      (`MeshComponent.SetScalarParameterValueOnMaterials` (`self.obraz2`) "Glow Int" 0.0)
      (set `self.Index` -1)
      (`self.DisableInput` (`GameplayStatics.GetPlayerController` 0)))))

(event `self.coll3.OnComponentBeginOverlap`
  (params (OverlappedComponent :type "PrimitiveComponent Object Reference") (OtherActor :type "Actor Object Reference") (OtherComp :type "PrimitiveComponent Object Reference") (OtherBodyIndex :type Integer) (bFromSweep :type Boolean) (SweepResult :type "HitResult Structure (by ref)"))
  (if (== OtherActor (`self.As BP First Person Character`))
    (if (not (`self.Solved?`))
      (`SceneComponent.SetVisibility` (`self.Widget3`) true false)
      (`MeshComponent.SetScalarParameterValueOnMaterials` (`self.obraz3`) "Glow Int" 1.0)
      (set `self.Index` 2)
      (`self.EnableInput` (`GameplayStatics.GetPlayerController` 0)))))

(event `self.coll3.OnComponentEndOverlap`
  (params (OverlappedComponent :type "PrimitiveComponent Object Reference") (OtherActor :type "Actor Object Reference") (OtherComp :type "PrimitiveComponent Object Reference") (OtherBodyIndex :type Integer))
  (if (== (`self.As BP First Person Character`) OtherActor)
    (if (not (`self.Solved?`))
      (`SceneComponent.SetVisibility` (`self.Widget3`) false false)
      (`MeshComponent.SetScalarParameterValueOnMaterials` (`self.obraz3`) "Glow Int" 0.0)
      (set `self.Index` -1)
      (`self.DisableInput` (`GameplayStatics.GetPlayerController` 0)))))

(event `self.coll4.OnComponentBeginOverlap`
  (params (OverlappedComponent :type "PrimitiveComponent Object Reference") (OtherActor :type "Actor Object Reference") (OtherComp :type "PrimitiveComponent Object Reference") (OtherBodyIndex :type Integer) (bFromSweep :type Boolean) (SweepResult :type "HitResult Structure (by ref)"))
  (if (== OtherActor (`self.As BP First Person Character`))
    (if (not (`self.Solved?`))
      (`SceneComponent.SetVisibility` (`self.Widget4`) true false)
      (`MeshComponent.SetScalarParameterValueOnMaterials` (`self.obraz4`) "Glow Int" 1.0)
      (set `self.Index` 3)
      (`self.EnableInput` (`GameplayStatics.GetPlayerController` 0)))))

(event `self.coll4.OnComponentEndOverlap`
  (params (OverlappedComponent :type "PrimitiveComponent Object Reference") (OtherActor :type "Actor Object Reference") (OtherComp :type "PrimitiveComponent Object Reference") (OtherBodyIndex :type Integer))
  (if (== (`self.As BP First Person Character`) OtherActor)
    (if (not (`self.Solved?`))
      (`SceneComponent.SetVisibility` (`self.Widget4`) false false)
      (`MeshComponent.SetScalarParameterValueOnMaterials` (`self.obraz4`) "Glow Int" 0.0)
      (set `self.Index` -1)
      (`self.DisableInput` (`GameplayStatics.GetPlayerController` 0)))))

(event `RotatePainting`
  (bind (_selectedpaintingtrans_location _selectedpaintingtrans_rotation _selectedpaintingtrans_scale) (`KismetMathLibrary.BreakTransform` (`self.SelectedPaintingTrans`)))
  (bind _setlectedpainting (`self.setlectedPainting`))
  (bind _index (`self.Index`))
  (bind _currentrotation (`self.CurrentRotation`))
  (bind _index_2 (`self.Index`))
  (bind _currentrotation_2 (`self.CurrentRotation`))
  (bind _returnvalue (`SceneComponent.K2_GetComponentToWorld` _setlectedpainting))
  (bind _returnvalue_2 (`KismetMathLibrary.MakeRotator` (`KismetMathLibrary.Conv_IntToDouble` (`KismetMathLibrary.Round` (.roll (.rotation _returnvalue)))) (`KismetMathLibrary.Conv_IntToDouble` (`KismetMathLibrary.Round` (.pitch (.rotation _returnvalue)))) (`KismetMathLibrary.Conv_IntToDouble` (`KismetMathLibrary.Round` (.yaw (.rotation _returnvalue))))))
  (set `self.canMove?` false)
  (switch `int` (`self.Index`)
    (:`0`
      (set `self.SelectedPaintingTrans` (`SceneComponent.K2_GetComponentToWorld` (`self.obraz1`)))
      (set `self.setlectedPainting` (`self.obraz1`))
      (bind (_direction _newtrack_0) (`Timeline|Rotate` :!via `PlayFromStart` :!label _label)
        (:`Update`
          (`SceneComponent.K2_SetWorldTransform` _setlectedpainting (`KismetMathLibrary.MakeTransform` _selectedpaintingtrans_location (`KismetMathLibrary.RLerp` _selectedpaintingtrans_rotation (`KismetMathLibrary.ComposeRotators` _selectedpaintingtrans_rotation (struct :`Pitch` 90.0)) _newtrack_0) _selectedpaintingtrans_scale) false false))
        (:`Finished`
          (switch `int` (`self.Index`)
            (:`0`
              (`KismetArrayLibrary.Array_Set` _currentrotation_2 _index_2 _returnvalue_2))
            (:`1`
              (`KismetArrayLibrary.Array_Set` _currentrotation_2 _index_2 _returnvalue_2))
            (:`2`
              (`KismetArrayLibrary.Array_Set` _currentrotation _index _returnvalue_2))
            (:`3`
              (`KismetArrayLibrary.Array_Set` _currentrotation _index _returnvalue_2)))
          (`self.CheckIfGood`))))
    (:`1`
      (set `self.SelectedPaintingTrans` (`SceneComponent.K2_GetComponentToWorld` (`self.obraz2`)))
      (set `self.setlectedPainting` (`self.obraz2`))
      (goto _label :!via `PlayFromStart`))
    (:`2`
      (set `self.SelectedPaintingTrans` (`SceneComponent.K2_GetComponentToWorld` (`self.obraz3`)))
      (set `self.setlectedPainting` (`self.obraz3`))
      (goto _label :!via `PlayFromStart`))
    (:`3`
      (set `self.SelectedPaintingTrans` (`SceneComponent.K2_GetComponentToWorld` (`self.obraz4`)))
      (set `self.setlectedPainting` (`self.obraz4`))
      (goto _label :!via `PlayFromStart`))))

(event `EnhancedInput|/Game/FirstPerson/Input/Actions/IA_Interact`
  (params (ActionValue :type Boolean) (ElapsedSeconds :type "Float (double-precision)") (TriggeredSeconds :type "Float (double-precision)") (InputAction :type "InputAction Object Reference" :default "/Game/FirstPerson/Input/Actions/IA_Interact.IA_Interact"))
  (:`Started`
    (if (`self.canMove?`)
      (`self.RotatePainting`))))

(event `CheckIfGood`
  (set `self.CorrectCount` 0)
  (for (_array_element _array_index) (`self.CurrentRotation`)
    (if (== (`|GetArrayItem` (`self.CorrectRotation`) _array_index) _array_element :`ErrorTolerance` 0.1)
      (`/Engine/EditorBlueprintResources/StandardMacros.IncrementInt` (`self.CorrectCount`)
        (:`  `
          (switch `int` _array_index
            (:`0`
              (`/Game/Game_Assets/HouseMeshes/House/2Floor/candlePuzzle/BP_candle.TurnOffcandle` (`self.candelref1`)))
            (:`1`
              (`/Game/Game_Assets/HouseMeshes/House/2Floor/candlePuzzle/BP_candle.TurnOffcandle` (`self.candelref2`)))
            (:`2`
              (`/Game/Game_Assets/HouseMeshes/House/2Floor/candlePuzzle/BP_candle.TurnOffcandle` (`self.candelref3`)))
            (:`3`
              (`/Game/Game_Assets/HouseMeshes/House/2Floor/candlePuzzle/BP_candle.TurnOffcandle` (`self.candelref4`))))))))
  (if (== (`self.CorrectCount`) 4)
    (`SceneComponent.SetVisibility` (`self.Widget1`) false false)
    (`SceneComponent.SetVisibility` (`self.Widget3`) false false)
    (`SceneComponent.SetVisibility` (`self.Widget2`) false false)
    (`SceneComponent.SetVisibility` (`self.Widget4`) false false)
    (`MeshComponent.SetScalarParameterValueOnMaterials` (`self.Widget4`) "Glow Int" 0.0)
    (`MeshComponent.SetScalarParameterValueOnMaterials` (`self.Widget2`) "Glow Int" 0.0)
    (`MeshComponent.SetScalarParameterValueOnMaterials` (`self.Widget3`) "Glow Int" 0.0)
    (`MeshComponent.SetScalarParameterValueOnMaterials` (`self.Widget1`) "Glow Int" 0.0)
    (set `self.Solved?` true)
    (`/Game/Game_Assets/HouseMeshes/House/2Floor/candlePuzzle/BP_LastPainting.Attachkey&Move` (`self.PaintingRef`))
    (else
      (set `self.canMove?` true))))

(fn `UserConstructionScript`)