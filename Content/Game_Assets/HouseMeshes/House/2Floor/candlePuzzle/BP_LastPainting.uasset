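; Final painting actor in the house's candle puzzle, which rotates the painting and places a key on it.
; The Attachkey&Move event plays the Move timeline, lerping Obraz3 to a fixed rotation along the shortest path.
; When the timeline finishes, it snaps the referenced key to a socket on the Plane component and prints the key's transform.
; BeginPlay also enables player input on the actor.
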(event `self.ReceiveBeginPlay`
  (`self.EnableInput` (`GameplayStatics.GetPlayerController` 0)))

(event `Attachkey&Move`
  (bind (_transf_location _transf_rotation _transf_scale) (`KismetMathLibrary.BreakTransform` (`self.Transf`)))
  (set `self.Transf` (`SceneComponent.K2_GetComponentToWorld` (`self.obraz3`)))
  (bind (_direction _newtrack_0) (`Timeline|Move`)
    (:`Update`
      (`SceneComponent.K2_SetWorldTransform` (`self.obraz3`) (`KismetMathLibrary.MakeTransform` _transf_location (`KismetMathLibrary.RLerp` _transf_rotation (struct :`Yaw` 330.0 :`Roll` 90.0) _newtrack_0 true) _transf_scale) false false))
    (:`Finished`
      (`self.K2_AttachToComponent` (`self.KeyRef`) (`self.Plane`) "Socket" "SnapToTarget" "SnapToTarget" "SnapToTarget" true)
      (`KismetSystemLibrary.PrintString` (`KismetStringLibrary.Conv_TransformToString` (`SceneComponent.K2_GetComponentToWorld` (`/Game/Game_Assets/HouseMeshes/House/2Floor/candlePuzzle/BP_FlashleyLAST.Key` (`self.KeyRef`))))))))

(fn `UserConstructionScript`)