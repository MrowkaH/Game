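; BP_DoorBarrs is a barred door that the first-person player opens with a key.
; Overlapping its Coll component shows a prompt widget and enables input on the actor; leaving hides it and disables input.
; On IA_Interact, a held key is deleted and a timeline rotates the bars open on yaw while destroying Coll.
; Without a key, it only prints a Polish "no key" debug message.
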(event `self.ReceiveBeginPlay`
  (bind _asbp_first_person_character (cast `/Game/FirstPerson/Blueprints/BP_FirstPersonCharacter` (`GameplayStatics.GetPlayerCharacter` 0)))
  (set `self.As BP First Person Character` _asbp_first_person_character))

(event `self.Coll.OnComponentBeginOverlap`
  (params (OverlappedComponent :type "PrimitiveComponent Object Reference") (OtherActor :type "Actor Object Reference") (OtherComp :type "PrimitiveComponent Object Reference") (OtherBodyIndex :type Integer) (bFromSweep :type Boolean) (SweepResult :type "HitResult Structure (by ref)"))
  (if (== OtherActor (`self.As BP First Person Character`))
    (`SceneComponent.SetVisibility` (`self.Widget`) true false)
    (`self.EnableInput` (`GameplayStatics.GetPlayerController` 0))))

(event `self.Coll.OnComponentEndOverlap`
  (params (OverlappedComponent :type "PrimitiveComponent Object Reference") (OtherActor :type "Actor Object Reference") (OtherComp :type "PrimitiveComponent Object Reference") (OtherBodyIndex :type Integer))
  (if (== OtherActor (`self.As BP First Person Character`))
    (`SceneComponent.SetVisibility` (`self.Widget`) false false)
    (`self.DisableInput` (`GameplayStatics.GetPlayerController` 0))))

(event `EnhancedInput|/Game/FirstPerson/Input/Actions/IA_Interact`
  (params (ActionValue :type Boolean) (ElapsedSeconds :type "Float (double-precision)") (TriggeredSeconds :type "Float (double-precision)") (InputAction :type "InputAction Object Reference" :default "/Game/FirstPerson/Input/Actions/IA_Interact.IA_Interact"))
  (:`Started`
    (if (`/Game/FirstPerson/Blueprints/BP_FirstPersonCharacter.HasKey?` (`self.As BP First Person Character`))
      (`/Game/FirstPerson/Blueprints/BP_FirstPersonCharacter.DeleteKey` (`self.As BP First Person Character`))
      (bind (_direction _open_close) (`Timeline|Door`)
        (:`Update`
          (`SceneComponent.K2_SetRelativeRotation` (`self.Bars`) (`KismetMathLibrary.MakeRotator` 0.0 0.0 (`KismetMathLibrary.Lerp` 0.0 -100.0 _open_close)) false false)
          (`ActorComponent.K2_DestroyComponent` (`self.Coll`))))
      (else
        (`KismetSystemLibrary.PrintString` "Brak klucza")))))

(fn `UserConstructionScript`)