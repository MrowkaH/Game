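; BP_FlashleyLvl2 is a key item that tells its linked Door to open when PickUpKey fires.
; While Action is set through the Opened event, the player entering BigCol shows the Info component, makes the Key material glow and enables input on the actor.
; Leaving BigCol hides Info and turns off the glow, but input stays enabled.
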(event `self.ReceiveBeginPlay`
  (bind _asbp_first_person_character (cast `/Game/FirstPerson/Blueprints/BP_FirstPersonCharacter` (`GameplayStatics.GetPlayerCharacter` 0)))
  (set `self.As BP First Person Character` _asbp_first_person_character)
  (`SceneComponent.K2_AttachToComponent` (`self.Info`) (`self.Key`) "None" "SnapToTarget" "KeepRelative" "KeepRelative" true))

(event `self.bigCol.OnComponentBeginOverlap`
  (params (OverlappedComponent :type "PrimitiveComponent Object Reference") (OtherActor :type "Actor Object Reference") (OtherComp :type "PrimitiveComponent Object Reference") (OtherBodyIndex :type Integer) (bFromSweep :type Boolean) (SweepResult :type "HitResult Structure (by ref)"))
  (if (== OtherActor (`self.As BP First Person Character`))
    (if (`self.Action?`)
      (`SceneComponent.SetVisibility` (`self.Info`) true false)
      (`MeshComponent.SetScalarParameterValueOnMaterials` (`self.Key`) "Glow Intensity" 1.0)
      (`self.EnableInput` (`GameplayStatics.GetPlayerController` 0)))))

(event `self.bigCol.OnComponentEndOverlap`
  (params (OverlappedComponent :type "PrimitiveComponent Object Reference") (OtherActor :type "Actor Object Reference") (OtherComp :type "PrimitiveComponent Object Reference") (OtherBodyIndex :type Integer))
  (if (== OtherActor (`self.As BP First Person Character`))
    (`SceneComponent.SetVisibility` (`self.Info`) false false)
    (`MeshComponent.SetScalarParameterValueOnMaterials` (`self.Key`) "Glow Intensity" 0.0)))

(event `self.PickUpKey`
  (message `/Game/Game_Assets/Scripts/Items/BPI_Door.OpenDoors` (`self.Door`)))

(event `/Game/test/Mebloscianka/BPI_MBKeyToOpen.Opened`
  (params (`ActionCompleted?` :type "Boolean (by ref)"))
  (set `self.Action?` `ActionCompleted?`))

(fn `UserConstructionScript`)