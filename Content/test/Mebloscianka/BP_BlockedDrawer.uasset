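; Blocked drawer that the player pries open with a crowbar, showing a prompt widget while they overlap its trigger.
; Open takes the held item, locks movement and look, then chains timelines to move the crowbar to a wave point, jiggle it, slide the drawer out and return the crowbar.
; Without a crowbar, the drawer only jiggles and a temporary "can't open" widget appears.
; Success restores control, calls Opened and removes the trigger.
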(event `self.ReceiveBeginPlay`
  (bind _asbp_first_person_character (cast `/Game/FirstPerson/Blueprints/BP_FirstPersonCharacter` (`GameplayStatics.GetPlayerCharacter` 0)))
  (set `self.As BP First Person Character` _asbp_first_person_character)
  (set `self.Original Loc` (`SceneComponent.K2_GetComponentLocation` (`self.Back`)))
  (set `self.WPTransform` (`SceneComponent.K2_GetComponentToWorld` (`self.WavePoint`))))

(event `self.coll.OnComponentBeginOverlap`
  (params (OverlappedComponent :type "PrimitiveComponent Object Reference") (OtherActor :type "Actor Object Reference") (OtherComp :type "PrimitiveComponent Object Reference") (OtherBodyIndex :type Integer) (bFromSweep :type Boolean) (SweepResult :type "HitResult Structure (by ref)"))
  (if (`self.Opened?`)
    _
    (elif (== OtherActor (`self.As BP First Person Character`))
      (`SceneComponent.SetVisibility` (`self.Widget`) true false)
      (set `self.CanOpen?` true))))

(event `self.coll.OnComponentEndOverlap`
  (params (OverlappedComponent :type "PrimitiveComponent Object Reference") (OtherActor :type "Actor Object Reference") (OtherComp :type "PrimitiveComponent Object Reference") (OtherBodyIndex :type Integer))
  (if (`self.Opened?`)
    _
    (elif (== (`self.As BP First Person Character`) OtherActor)
      (`SceneComponent.SetVisibility` (`self.Widget`) false false)
      (set `self.CanOpen?` false))))

(event `/Game/test/Mebloscianka/BPI_MBKeyToOpen.Open`
  (params (`hasCrowbar?` :type "Boolean (by ref)") (HeldItem :type "Actor Object Reference (by ref)"))
  (bind (_original_loc_x _original_loc_y _original_loc_z) (`KismetMathLibrary.BreakVector` (`self.Original Loc`)))
  (bind _crowbarloc (`self.CrowbarLoc`))
  (bind (_crowbarloc_location _crowbarloc_rotation _crowbarloc_scale) (`KismetMathLibrary.BreakTransform` (`self.CrowbarLoc`)))
  (bind (_crowbarloc_location_2 _crowbarloc_rotation_2 _crowbarloc_scale_2) (`KismetMathLibrary.BreakTransform` (`self.CrowbarLoc`)))
  (bind (_wptransform_location _wptransform_rotation) (`KismetMathLibrary.BreakTransform` (`self.WPTransform`)))
  (bind (_crowbaroriginalloc_location _crowbaroriginalloc_rotation) (`KismetMathLibrary.BreakTransform` (`self.CrowbarOriginalLoc`)))
  (bind (_crowbarloc_location_3 _crowbarloc_rotation_3 _crowbarloc_scale_3) (`KismetMathLibrary.BreakTransform` (`self.CrowbarLoc`)))
  (bind (_original_loc_x_2 _original_loc_y_2 _original_loc_z_2) (`KismetMathLibrary.BreakVector` (`self.Original Loc`)))
  (bind _output_get (set `self.Held Item` HeldItem))
  (bind _output_get_2 (set `self.Has Crowbar?` `hasCrowbar?`))
  (if (`self.Opened?`)
    _
    (elif _output_get_2
      (bind _returnvalue (`self.GetTransform` _output_get))
      (set `self.CrowbarLoc` _returnvalue)
      (set `self.CrowbarOriginalLoc` _returnvalue)
      (`CharacterMovementComponent.DisableMovement` (`Character.CharacterMovement` (`self.As BP First Person Character`)))
      (`Controller.SetIgnoreLookInput` (`GameplayStatics.GetPlayerController` 0) true)
      (bind (_direction _newtrack_0) (`Timeline|openDrawer`)
        (:`Update`
          (bind _returnvalue_2 (`KismetMathLibrary.VLerp` _crowbarloc_location_2 _wptransform_location _newtrack_0))
          (bind _returnvalue_3 (`KismetMathLibrary.RLerp` _crowbarloc_rotation_2 _wptransform_rotation _newtrack_0))
          (`SceneComponent.K2_SetWorldTransform` (`Actor.RootComponent` (`self.Held Item`)) (`KismetMathLibrary.MakeTransform` _returnvalue_2 _returnvalue_3 _crowbarloc_scale_2) false false)
          (set `self.CrowbarLoc` (`KismetMathLibrary.MakeTransform` _returnvalue_2 _returnvalue_3 _crowbarloc_scale_2)))
        (:`Finished`
          (bind (_direction_2 _move) (`Timeline|Timeline` :!label _label)
            (:`Update`
              (`SceneComponent.K2_SetWorldTransform` (`self.Back`) (`KismetMathLibrary.MakeTransform` (`KismetMathLibrary.VLerp` (`self.Original Loc`) (`KismetMathLibrary.MakeVector` _original_loc_x _original_loc_y (+ _original_loc_z 0.5)) _move)) false false)
              (if (`self.Has Crowbar?`)
                (bind (_direction_3 _move_2) (`Timeline|Timeline_0`)
                  (:`Update`
                    (`SceneComponent.K2_SetWorldTransform` (`Actor.RootComponent` (`self.Held Item`)) (`KismetMathLibrary.MakeTransform` (`KismetMathLibrary.VLerp` _crowbarloc_location (`KismetMathLibrary.MakeVector` (- (.x (.location _crowbarloc)) 0.3) (.y (.location _crowbarloc)) (+ (.z (.location _crowbarloc)) 0.5)) _move_2) (`KismetMathLibrary.RLerp` _crowbarloc_rotation) _crowbarloc_scale) false false)))
                (else
                  (`/Engine/EditorBlueprintResources/StandardMacros.DoOnce` false :!label _label_2
                    (:`Completed`
                      (bind _returnvalue_4 (`|CreateWidget` "/Game/test/Notatki/BPW_CantOpen.BPW_CantOpen_C"))
                      (`UserWidget.AddToViewport` _returnvalue_4 0)
                      (`Widget.SetVisibility` _returnvalue_4 "Visible")
                      (`KismetSystemLibrary.Delay` 2.0)
                      (`Widget.SetVisibility` _returnvalue_4 "Hidden")
                      (goto _label_2 :!via `Reset`))))))
            (:`Finished`
              (if (`self.Has Crowbar?`)
                (bind (_direction_4 _move_3) (`Timeline|Move`)
                  (:`Update`
                    (bind _returnvalue_5 (`KismetMathLibrary.VLerp` (`self.Original Loc`) (`KismetMathLibrary.MakeVector` (+ _original_loc_x_2 45.0) _original_loc_y_2 _original_loc_z_2) _move_3))
                    (`SceneComponent.K2_SetWorldTransform` (`self.Back`) (`KismetMathLibrary.MakeTransform` _returnvalue_5) false false)
                    (bind (_direction_5 _newtrack_0_2) (`Timeline|Timeline_1`)
                      (:`Update`
                        (`SceneComponent.K2_SetWorldTransform` (`Actor.RootComponent` (`self.Held Item`)) (`KismetMathLibrary.MakeTransform` (`KismetMathLibrary.VLerp` _crowbarloc_location_3 _crowbaroriginalloc_location _newtrack_0_2) (`KismetMathLibrary.RLerp` _crowbarloc_rotation_3 _crowbaroriginalloc_rotation _newtrack_0_2) _crowbarloc_scale_3) false false))))
                  (:`Finished`
                    (set `self.Original Loc` _returnvalue_5)
                    (`CharacterMovementComponent.SetMovementMode` (`Character.CharacterMovement` (`GameplayStatics.GetPlayerCharacter` 0)) "MOVE_Walking" 0)
                    (`Controller.ResetIgnoreLookInput` (`PlayerState.GetPlayerController` (`Pawn.PlayerState` (`self.As BP First Person Character`))))
                    (bind _output_get_3 (set `self.Opened?` true))
                    (`/Game/test/Mebloscianka/BPI_MBKeyToOpen.Opened` _output_get_3)
                    (`SceneComponent.SetVisibility` (`self.Widget`) false false)
                    (`ActorComponent.K2_DestroyComponent` (`self.coll`)))))))))
      (else
        (goto _label :!via `PlayFromStart`)))))

(fn `UserConstructionScript`)