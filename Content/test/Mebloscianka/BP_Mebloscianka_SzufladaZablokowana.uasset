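; Locked drawer (Szuflada) in a wall unit that only jiggles instead of opening.
; The Coll overlap lets the first-person player interact by toggling a widget, player input and the CanOpen flag, with debug prints.
; While CanOpen is set, TLShake plays the Move timeline, which lerps the drawer between its BeginPlay location and a point slightly above it.
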(event `self.ReceiveBeginPlay`
  (bind _asbp_first_person_character (cast `/Game/FirstPerson/Blueprints/BP_FirstPersonCharacter` (`GameplayStatics.GetPlayerCharacter` 0)))
  (set `self.As BP First Person Character` _asbp_first_person_character)
  (set `self.OriginalLoc` (`SceneComponent.K2_GetComponentLocation` (`self.szuflada`))))

(event `self.coll.OnComponentBeginOverlap`
  (params (OverlappedComponent :type "PrimitiveComponent Object Reference") (OtherActor :type "Actor Object Reference") (OtherComp :type "PrimitiveComponent Object Reference") (OtherBodyIndex :type Integer) (bFromSweep :type Boolean) (SweepResult :type "HitResult Structure (by ref)"))
  (if (== OtherActor (`self.As BP First Person Character`))
    (`SceneComponent.SetVisibility` (`self.Widget`) true false)
    (set `self.canOpen?` true)
    (`KismetSystemLibrary.PrintString` "canopen")
    (`self.EnableInput` (`GameplayStatics.GetPlayerController` 0))))

(event `self.coll.OnComponentEndOverlap`
  (params (OverlappedComponent :type "PrimitiveComponent Object Reference") (OtherActor :type "Actor Object Reference") (OtherComp :type "PrimitiveComponent Object Reference") (OtherBodyIndex :type Integer))
  (if (== (`self.As BP First Person Character`) OtherActor)
    (`SceneComponent.SetVisibility` (`self.Widget`) false false)
    (set `self.canOpen?` false)
    (`KismetSystemLibrary.PrintString` "cantopen")
    (`self.DisableInput` (`GameplayStatics.GetPlayerController` 0))))

(event `/Game/Game_Assets/Scripts/Items/BPI_Mebl.TLShake`
  (bind (_originalloc_x _originalloc_y _originalloc_z) (`KismetMathLibrary.BreakVector` (`self.OriginalLoc`)))
  (if (`self.canOpen?`)
    (bind (_direction _move) (`Timeline|Move` :!via `PlayFromStart`)
      (:`Update`
        (`SceneComponent.K2_SetWorldTransform` (`self.szuflada`) (`KismetMathLibrary.MakeTransform` (`KismetMathLibrary.VLerp` (`self.OriginalLoc`) (`KismetMathLibrary.MakeVector` _originalloc_x _originalloc_y (+ _originalloc_z 0.5)) _move)) false false)))))

(fn `UserConstructionScript`)