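; Unlocked drawer that the player can slide open and closed when standing within its trigger.
; The collision overlap with the first-person character shows a widget and sets a flag that allows the Open event to act.
; Open uses a FlipFlop to play or reverse a timeline that lerps the Back component from its BeginPlay location along negative world Y, so the slide ignores the drawer's facing.
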(event `self.ReceiveBeginPlay`
  (bind _back (`self.Back`))
  (set `self.Original Loc` (`SceneComponent.K2_GetComponentLocation` _back))
  (set `self.rotator` (`SceneComponent.K2_GetComponentRotation` _back)))

(event `self.coll.OnComponentBeginOverlap`
  (params (OverlappedComponent :type "PrimitiveComponent Object Reference") (OtherActor :type "Actor Object Reference") (OtherComp :type "PrimitiveComponent Object Reference") (OtherBodyIndex :type Integer) (bFromSweep :type Boolean) (SweepResult :type "HitResult Structure (by ref)"))
  (bind _asbp_first_person_character (cast `/Game/FirstPerson/Blueprints/BP_FirstPersonCharacter` (`GameplayStatics.GetPlayerCharacter` 0)))
  (set `self.As BP First Person Character` _asbp_first_person_character)
  (if (== OtherActor (`self.As BP First Person Character`))
    (`SceneComponent.SetVisibility` (`self.Widget`) true false)
    (set `self.CanOpen?` true)))

(event `self.coll.OnComponentEndOverlap`
  (params (OverlappedComponent :type "PrimitiveComponent Object Reference") (OtherActor :type "Actor Object Reference") (OtherComp :type "PrimitiveComponent Object Reference") (OtherBodyIndex :type Integer))
  (if (== (`self.As BP First Person Character`) OtherActor)
    (`SceneComponent.SetVisibility` (`self.Widget`) false false)
    (set `self.CanOpen?` false)))

(event `self.Open`
  (params (`hasCrowbar?` :type "Boolean (by ref)") (HeldItem :type "Actor Object Reference (by ref)"))
  (bind (_original_loc_x _original_loc_y _original_loc_z) (`KismetMathLibrary.BreakVector` (`self.Original Loc`)))
  (if (`self.CanOpen?`)
    (`/Engine/EditorBlueprintResources/StandardMacros.FlipFlop`
      (:`A`
        (bind (_direction _move) (`Timeline|Move` :!label _label)
          (:`Update`
            (`SceneComponent.K2_SetWorldTransform` (`self.Back`) (`KismetMathLibrary.MakeTransform` (`KismetMathLibrary.VLerp` (`self.Original Loc`) (`KismetMathLibrary.MakeVector` _original_loc_x (+ _original_loc_y -45.0) _original_loc_z) _move) (`self.rotator`)) false false))))
      (:`B`
        (goto _label :!via `Reverse`)))))

(fn `UserConstructionScript`)