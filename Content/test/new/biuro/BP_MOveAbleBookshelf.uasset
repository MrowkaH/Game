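; Interactable bookshelf actor that the first-person player pushes aside once.
; Box overlap shows a prompt widget and arms IA_Interact while the player is inside.
; Interacting calls ChangeLight on a referenced lamp, disables movement, switches input mode and attaches the player to Ref with world transform kept.
; A timeline slides the mesh 45 units along negative world Y, then restores walking and game-only input and marks it pushed.
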(event `self.ReceiveBeginPlay`
  (set `self.ShelfTrans` (`SceneComponent.K2_GetComponentToWorld` (`self.Plane_003`))))

(event `self.Box.OnComponentBeginOverlap`
  (params (OverlappedComponent :type "PrimitiveComponent Object Reference") (OtherActor :type "Actor Object Reference") (OtherComp :type "PrimitiveComponent Object Reference") (OtherBodyIndex :type Integer) (bFromSweep :type Boolean) (SweepResult :type "HitResult Structure (by ref)"))
  (bind _asbp_first_person_character (cast `/Game/FirstPerson/Blueprints/BP_FirstPersonCharacter` (`GameplayStatics.GetPlayerCharacter` 0)))
  (set `self.As BP First Person Character` _asbp_first_person_character)
  (if (== OtherActor (`self.As BP First Person Character`))
    (if (not (`self.Pushed?`))
      (`SceneComponent.SetVisibility` (`self.Widget`) true false)
      (`self.EnableInput` (`GameplayStatics.GetPlayerController` 0))
      (set `self.CanMove?` true))))

(event `self.Box.OnComponentEndOverlap`
  (params (OverlappedComponent :type "PrimitiveComponent Object Reference") (OtherActor :type "Actor Object Reference") (OtherComp :type "PrimitiveComponent Object Reference") (OtherBodyIndex :type Integer))
  (if (== (`self.As BP First Person Character`) OtherActor)
    (`SceneComponent.SetVisibility` (`self.Widget`) false false)
    (set `self.CanMove?` false)))

(event `EnhancedInput|/Game/FirstPerson/Input/Actions/IA_Interact`
  (params (ActionValue :type Boolean) (ElapsedSeconds :type "Float (double-precision)") (TriggeredSeconds :type "Float (double-precision)") (InputAction :type "InputAction Object Reference" :default "/Game/FirstPerson/Input/Actions/IA_Interact.IA_Interact"))
  (bind _returnvalue (`GameplayStatics.GetPlayerController` 0))
  (:`Started`
    (if (`self.CanMove?`)
      (`self.moveShelf`)
      (`/Game/test/new/lamp/BP_LampUP.ChangeLight` (`self.LampRef`))
      (`CharacterMovementComponent.DisableMovement` (`Character.CharacterMovement` (`GameplayStatics.GetPlayerCharacter` 0)))
      (`Controller.SetIgnoreLookInput` _returnvalue false)
      (`WidgetBlueprintLibrary.SetInputMode_GameAndUIEx` _returnvalue null "LockAlways")
      (`self.PlayerControl`))))

(event `moveShelf`
  (bind _returnvalue (`GameplayStatics.GetPlayerController` 0))
  (bind (_shelftrans_location _shelftrans_rotation _shelftrans_scale) (`KismetMathLibrary.BreakTransform` (`self.ShelfTrans`)))
  (bind _shelftrans (`self.ShelfTrans`))
  (if (not (`self.Pushed?`))
    (bind (_direction _newtrack_0) (`Timeline|Timeline` :!via `PlayFromStart`)
      (:`Update`
        (`SceneComponent.K2_SetWorldTransform` (`self.Plane_003`) (`KismetMathLibrary.MakeTransform` (`KismetMathLibrary.VLerp` _shelftrans_location (`KismetMathLibrary.MakeVector` (.x (.location _shelftrans)) (+ (.y (.location _shelftrans)) -45.0) (.z (.location _shelftrans))) _newtrack_0) _shelftrans_rotation _shelftrans_scale) false false))
      (:`Finished`
        (`CharacterMovementComponent.SetMovementMode` (`Character.CharacterMovement` (`GameplayStatics.GetPlayerCharacter` 0)) "MOVE_Walking" 0)
        (`Controller.ResetIgnoreLookInput` _returnvalue)
        (`WidgetBlueprintLibrary.SetInputMode_GameOnly` _returnvalue)
        (set `self.Pushed?` true)))))

(fn `PlayerControl`
  (`self.K2_AttachToComponent` (`GameplayStatics.GetPlayerCharacter` 0) (`self.ref`) "None" "KeepWorld" "KeepWorld" "KeepWorld" true))

(fn `UserConstructionScript`)