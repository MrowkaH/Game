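; Coffin ("trumna") puzzle actor with six toggleable handles that opens its lid and presents a key when solved.
; Per-handle overlap boxes show a widget, enable input and set the focused handle; interact toggles its state and animates it by timeline.
; Switching a handle on compares states to the correct pattern; a match swings the lid, then lifts and rotates the key after a delay.
; Handles 1, 3 and 5 get glowing gold materials at start.
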(event `self.ReceiveBeginPlay`
  (`SceneComponent.K2_SetRelativeRotation` (`self.moveablehandle6`) (struct :`Pitch` 70.0) false false)
  (`SceneComponent.K2_SetRelativeRotation` (`self.moveablehandle5`) (struct :`Pitch` 70.0) false false)
  (`SceneComponent.K2_SetRelativeRotation` (`self.moveablehandle4`) (struct :`Pitch` 70.0) false false)
  (`SceneComponent.K2_SetRelativeRotation` (`self.moveablehandle2`) (struct :`Pitch` 70.0) false false)
  (`SceneComponent.K2_SetRelativeRotation` (`self.moveablehandle1`) (struct :`Pitch` 70.0) false false)
  (`SceneComponent.K2_SetRelativeRotation` (`self.moveablehandle3`) (struct :`Pitch` 70.0) false false)
  (set `self.Spawn Transform` (`SceneComponent.K2_GetComponentToWorld` (`self.Ref`)))
  (bind _returnvalue (`PrimitiveComponent.CreateDynamicMaterialInstance` (`self.moveablehandle3`) 0 "/Game/Game_Assets/HouseMeshes/insinde/Trumna/Metallic_GoldGLowing_Inst.Metallic_GoldGLowing_Inst" "None"))
  (bind _returnvalue_2 (`PrimitiveComponent.CreateDynamicMaterialInstance` (`self.moveablehandle1`) 0 "/Game/Game_Assets/HouseMeshes/insinde/Trumna/Metallic_GoldGLowing_Inst.Metallic_GoldGLowing_Inst" "None"))
  (bind _returnvalue_3 (`PrimitiveComponent.CreateDynamicMaterialInstance` (`self.moveablehandle5`) 0 "/Game/Game_Assets/HouseMeshes/insinde/Trumna/Metallic_GoldGLowing_Inst.Metallic_GoldGLowing_Inst" "None"))
  (bind _output_get (set `self.HandleMaterials` (`|MakeArray` _returnvalue_3 _returnvalue_2 _returnvalue)))
  (for _array_element _output_get
    (`MaterialInstanceDynamic.SetScalarParameterValue` _array_element "ShouldGlow" 4.0)))

(event `checkpuzzle`
  (if (`KismetArrayLibrary.Array_Identical` (`self.CorrectState`) (`self.handleState`))
    (set `self.Opened?` true)
    (`self.MoveFlap`)))

(event `self.Box5.OnComponentBeginOverlap`
  (params (OverlappedComponent :type "PrimitiveComponent Object Reference") (OtherActor :type "Actor Object Reference") (OtherComp :type "PrimitiveComponent Object Reference") (OtherBodyIndex :type Integer) (bFromSweep :type Boolean) (SweepResult :type "HitResult Structure (by ref)"))
  (bind _asbp_first_person_character (cast `/Game/FirstPerson/Blueprints/BP_FirstPersonCharacter` (`GameplayStatics.GetPlayerCharacter` 0)))
  (set `self.As BP First Person Character` _asbp_first_person_character)
  (if (== OtherActor (`self.As BP First Person Character`))
    (`SceneComponent.SetVisibility` (`self.Widget5`) true false)
    (`self.EnableInput` (`GameplayStatics.GetPlayerController` 0))
    (set `self.FocusedHandle` 4)))

(event `self.Box5.OnComponentEndOverlap`
  (params (OverlappedComponent :type "PrimitiveComponent Object Reference") (OtherActor :type "Actor Object Reference") (OtherComp :type "PrimitiveComponent Object Reference") (OtherBodyIndex :type Integer))
  (if (== (`self.As BP First Person Character`) OtherActor)
    (`SceneComponent.SetVisibility` (`self.Widget5`) false false)
    (`self.DisableInput` (`GameplayStatics.GetPlayerController` 0))
    (set `self.FocusedHandle` -1)))

(event `self.Box6.OnComponentBeginOverlap`
  (params (OverlappedComponent :type "PrimitiveComponent Object Reference") (OtherActor :type "Actor Object Reference") (OtherComp :type "PrimitiveComponent Object Reference") (OtherBodyIndex :type Integer) (bFromSweep :type Boolean) (SweepResult :type "HitResult Structure (by ref)"))
  (bind _asbp_first_person_character (cast `/Game/FirstPerson/Blueprints/BP_FirstPersonCharacter` (`GameplayStatics.GetPlayerCharacter` 0)))
  (set `self.As BP First Person Character` _asbp_first_person_character)
  (if (== OtherActor (`self.As BP First Person Character`))
    (`SceneComponent.SetVisibility` (`self.Widget6`) true false)
    (`self.EnableInput` (`GameplayStatics.GetPlayerController` 0))
    (set `self.FocusedHandle` 5)))

(event `self.Box6.OnComponentEndOverlap`
  (params (OverlappedComponent :type "PrimitiveComponent Object Reference") (OtherActor :type "Actor Object Reference") (OtherComp :type "PrimitiveComponent Object Reference") (OtherBodyIndex :type Integer))
  (if (== (`self.As BP First Person Character`) OtherActor)
    (`SceneComponent.SetVisibility` (`self.Widget6`) false false)
    (`self.DisableInput` (`GameplayStatics.GetPlayerController` 0))
    (set `self.FocusedHandle` -1)))

(event `self.Box4.OnComponentBeginOverlap`
  (params (OverlappedComponent :type "PrimitiveComponent Object Reference") (OtherActor :type "Actor Object Reference") (OtherComp :type "PrimitiveComponent Object Reference") (OtherBodyIndex :type Integer) (bFromSweep :type Boolean) (SweepResult :type "HitResult Structure (by ref)"))
  (bind _asbp_first_person_character (cast `/Game/FirstPerson/Blueprints/BP_FirstPersonCharacter` (`GameplayStatics.GetPlayerCharacter` 0)))
  (set `self.As BP First Person Character` _asbp_first_person_character)
  (if (== OtherActor (`self.As BP First Person Character`))
    (`SceneComponent.SetVisibility` (`self.Widget4`) true false)
    (`self.EnableInput` (`GameplayStatics.GetPlayerController` 0))
    (set `self.FocusedHandle` 3)))

(event `self.Box4.OnComponentEndOverlap`
  (params (OverlappedComponent :type "PrimitiveComponent Object Reference") (OtherActor :type "Actor Object Reference") (OtherComp :type "PrimitiveComponent Object Reference") (OtherBodyIndex :type Integer))
  (if (== (`self.As BP First Person Character`) OtherActor)
    (`SceneComponent.SetVisibility` (`self.Widget4`) false false)
    (`self.DisableInput` (`GameplayStatics.GetPlayerController` 0))
    (set `self.FocusedHandle` -1)))

(event `self.Box2.OnComponentBeginOverlap`
  (params (OverlappedComponent :type "PrimitiveComponent Object Reference") (OtherActor :type "Actor Object Reference") (OtherComp :type "PrimitiveComponent Object Reference") (OtherBodyIndex :type Integer) (bFromSweep :type Boolean) (SweepResult :type "HitResult Structure (by ref)"))
  (bind _asbp_first_person_character (cast `/Game/FirstPerson/Blueprints/BP_FirstPersonCharacter` (`GameplayStatics.GetPlayerCharacter` 0)))
  (set `self.As BP First Person Character` _asbp_first_person_character)
  (if (== OtherActor (`self.As BP First Person Character`))
    (`SceneComponent.SetVisibility` (`self.Widget2`) true false)
    (`self.EnableInput` (`GameplayStatics.GetPlayerController` 0))
    (set `self.FocusedHandle` 1)))

(event `self.Box2.OnComponentEndOverlap`
  (params (OverlappedComponent :type "PrimitiveComponent Object Reference") (OtherActor :type "Actor Object Reference") (OtherComp :type "PrimitiveComponent Object Reference") (OtherBodyIndex :type Integer))
  (if (== (`self.As BP First Person Character`) OtherActor)
    (`SceneComponent.SetVisibility` (`self.Widget2`) false false)
    (`self.DisableInput` (`GameplayStatics.GetPlayerController` 0))
    (set `self.FocusedHandle` -1)))

(event `self.Box1.OnComponentBeginOverlap`
  (params (OverlappedComponent :type "PrimitiveComponent Object Reference") (OtherActor :type "Actor Object Reference") (OtherComp :type "PrimitiveComponent Object Reference") (OtherBodyIndex :type Integer) (bFromSweep :type Boolean) (SweepResult :type "HitResult Structure (by ref)"))
  (bind _asbp_first_person_character (cast `/Game/FirstPerson/Blueprints/BP_FirstPersonCharacter` (`GameplayStatics.GetPlayerCharacter` 0)))
  (set `self.As BP First Person Character` _asbp_first_person_character)
  (if (== OtherActor (`self.As BP First Person Character`))
    (`SceneComponent.SetVisibility` (`self.Widget1`) true false)
    (`self.EnableInput` (`GameplayStatics.GetPlayerController` 0))
    (set `self.FocusedHandle` 0)))

(event `self.Box1.OnComponentEndOverlap`
  (params (OverlappedComponent :type "PrimitiveComponent Object Reference") (OtherActor :type "Actor Object Reference") (OtherComp :type "PrimitiveComponent Object Reference") (OtherBodyIndex :type Integer))
  (if (== (`self.As BP First Person Character`) OtherActor)
    (`SceneComponent.SetVisibility` (`self.Widget1`) false false)
    (`self.DisableInput` (`GameplayStatics.GetPlayerController` 0))
    (set `self.FocusedHandle` -1)))

(event `self.Box3.OnComponentBeginOverlap`
  (params (OverlappedComponent :type "PrimitiveComponent Object Reference") (OtherActor :type "Actor Object Reference") (OtherComp :type "PrimitiveComponent Object Reference") (OtherBodyIndex :type Integer) (bFromSweep :type Boolean) (SweepResult :type "HitResult Structure (by ref)"))
  (bind _asbp_first_person_character (cast `/Game/FirstPerson/Blueprints/BP_FirstPersonCharacter` (`GameplayStatics.GetPlayerCharacter` 0)))
  (set `self.As BP First Person Character` _asbp_first_person_character)
  (if (== OtherActor (`self.As BP First Person Character`))
    (`SceneComponent.SetVisibility` (`self.Widget3`) true false)
    (`self.EnableInput` (`GameplayStatics.GetPlayerController` 0))
    (set `self.FocusedHandle` 2)))

(event `self.Box3.OnComponentEndOverlap`
  (params (OverlappedComponent :type "PrimitiveComponent Object Reference") (OtherActor :type "Actor Object Reference") (OtherComp :type "PrimitiveComponent Object Reference") (OtherBodyIndex :type Integer))
  (if (== (`self.As BP First Person Character`) OtherActor)
    (`SceneComponent.SetVisibility` (`self.Widget3`) false false)
    (`self.DisableInput` (`GameplayStatics.GetPlayerController` 0))
    (set `self.FocusedHandle` -1)))

(event `EnhancedInput|/Game/FirstPerson/Input/Actions/IA_Interact`
  (params (ActionValue :type Boolean) (ElapsedSeconds :type "Float (double-precision)") (TriggeredSeconds :type "Float (double-precision)") (InputAction :type "InputAction Object Reference" :default "/Game/FirstPerson/Input/Actions/IA_Interact.IA_Interact"))
  (bind _handlestate (`self.handleState`))
  (bind _focusedhandle (`self.FocusedHandle`))
  (bind _handlestate_2 (`self.handleState`))
  (bind _focusedhandle_2 (`self.FocusedHandle`))
  (bind _handlestate_3 (`self.handleState`))
  (bind _focusedhandle_3 (`self.FocusedHandle`))
  (bind _handlestate_4 (`self.handleState`))
  (bind _focusedhandle_4 (`self.FocusedHandle`))
  (bind _handlestate_5 (`self.handleState`))
  (bind _focusedhandle_5 (`self.FocusedHandle`))
  (bind _handlestate_6 (`self.handleState`))
  (bind _focusedhandle_6 (`self.FocusedHandle`))
  (:`Started`
    (switch `int` (`self.FocusedHandle`)
      (:`0`
        (`/Engine/EditorBlueprintResources/StandardMacros.FlipFlop`
          (:`A`
            (`KismetArrayLibrary.Array_Set` _handlestate_3 _focusedhandle_3 true)
            (`self.checkpuzzle`)
            (bind (_direction _newtrack_0) (`Timeline|Timeline` :!label _label)
              (:`Update`
                (`SceneComponent.K2_SetRelativeRotation` (`self.moveablehandle1`) (`KismetMathLibrary.RLerp` (struct :`Pitch` 70.0) (struct :`Pitch` 140.0) _newtrack_0) false false))))
          (:`B`
            (`KismetArrayLibrary.Array_Set` _handlestate_3 _focusedhandle_3)
            (goto _label :!via `Reverse`))))
      (:`1`
        (`/Engine/EditorBlueprintResources/StandardMacros.FlipFlop`
          (:`A`
            (`KismetArrayLibrary.Array_Set` _handlestate_2 _focusedhandle_2 true)
            (`self.checkpuzzle`)
            (bind (_direction_2 _newtrack_0_2) (`Timeline|Timeline_0` :!label _label_2)
              (:`Update`
                (`SceneComponent.K2_SetRelativeRotation` (`self.moveablehandle2`) (`KismetMathLibrary.RLerp` (struct :`Pitch` 70.0) (struct :`Pitch` 140.0) _newtrack_0_2) false false))))
          (:`B`
            (`KismetArrayLibrary.Array_Set` _handlestate_2 _focusedhandle_2)
            (goto _label_2 :!via `Reverse`))))
      (:`2`
        (`/Engine/EditorBlueprintResources/StandardMacros.FlipFlop`
          (:`A`
            (`KismetArrayLibrary.Array_Set` _handlestate_4 _focusedhandle_4 true)
            (`self.checkpuzzle`)
            (bind (_direction_3 _newtrack_0_3) (`Timeline|Timeline_1` :!via `PlayFromStart` :!label _label_3)
              (:`Update`
                (`SceneComponent.K2_SetRelativeRotation` (`self.moveablehandle3`) (`KismetMathLibrary.RLerp` (struct :`Pitch` 70.0) (struct :`Pitch` 140.0) _newtrack_0_3) false false))))
          (:`B`
            (`KismetArrayLibrary.Array_Set` _handlestate_4 _focusedhandle_4)
            (goto _label_3 :!via `Reverse`))))
      (:`3`
        (`/Engine/EditorBlueprintResources/StandardMacros.FlipFlop`
          (:`A`
            (`KismetArrayLibrary.Array_Set` _handlestate_5 _focusedhandle_5 true)
            (`self.checkpuzzle`)
            (bind (_direction_4 _newtrack_0_4) (`Timeline|Timeline_2` :!label _label_4)
              (:`Update`
                (`SceneComponent.K2_SetRelativeRotation` (`self.moveablehandle4`) (`KismetMathLibrary.RLerp` (struct :`Pitch` 70.0) (struct :`Pitch` 140.0) _newtrack_0_4) false false))))
          (:`B`
            (`KismetArrayLibrary.Array_Set` _handlestate_5 _focusedhandle_5)
            (goto _label_4 :!via `Reverse`))))
      (:`4`
        (`/Engine/EditorBlueprintResources/StandardMacros.FlipFlop`
          (:`A`
            (`KismetArrayLibrary.Array_Set` _handlestate_6 _focusedhandle_6 true)
            (`self.checkpuzzle`)
            (bind (_direction_5 _newtrack_0_5) (`Timeline|Timeline_3` :!label _label_5)
              (:`Update`
                (`SceneComponent.K2_SetRelativeRotation` (`self.moveablehandle5`) (`KismetMathLibrary.RLerp` (struct :`Pitch` 70.0) (struct :`Pitch` 140.0) _newtrack_0_5) false false))))
          (:`B`
            (`KismetArrayLibrary.Array_Set` _handlestate_6 _focusedhandle_6)
            (goto _label_5 :!via `Reverse`))))
      (:`5`
        (`/Engine/EditorBlueprintResources/StandardMacros.FlipFlop`
          (:`A`
            (`KismetArrayLibrary.Array_Set` _handlestate _focusedhandle true)
            (`self.checkpuzzle`)
            (bind (_direction_6 _newtrack_0_6) (`Timeline|Timeline_4` :!label _label_6)
              (:`Update`
                (`SceneComponent.K2_SetRelativeRotation` (`self.moveablehandle6`) (`KismetMathLibrary.RLerp` (struct :`Pitch` 70.0) (struct :`Pitch` 140.0) _newtrack_0_6) false false))))
          (:`B`
            (`KismetArrayLibrary.Array_Set` _handlestate _focusedhandle)
            (goto _label_6 :!via `Reverse`)))))))

(event `MoveFlap`
  (bind (_spawn_transform_location _spawn_transform_rotation) (`KismetMathLibrary.BreakTransform` (`self.Spawn Transform`)))
  (bind _spawn_transform (`self.Spawn Transform`))
  (bind (_direction _newtrack_0) (`Timeline|Timeline_5`)
    (:`Update`
      (`SceneComponent.K2_SetRelativeRotation` (`self.LId`) (`KismetMathLibrary.RLerp` (struct) (struct :`Pitch` 15.0) _newtrack_0) false false))
    (:`Finished`
      (`self.K2_AttachToComponent` (`self.KeyRef`) (`self.Ref`) "None" "KeepWorld" "KeepWorld" "KeepWorld" true)
      (`KismetSystemLibrary.Delay` 2.0)
      (bind (_direction_2 _newtrack_0_2) (`Timeline|Timeline_6`)
        (:`Update`
          (`SceneComponent.K2_SetWorldTransform` (`Actor.RootComponent` (`self.KeyRef`)) (`KismetMathLibrary.MakeTransform` (`KismetMathLibrary.VLerp` _spawn_transform_location (`KismetMathLibrary.MakeVector` (.x (.location _spawn_transform)) (.y (.location _spawn_transform)) (+ (.z (.location _spawn_transform)) 70.0)) _newtrack_0_2) (`KismetMathLibrary.RLerp` _spawn_transform_rotation (struct :`Pitch` -90.0) _newtrack_0_2)) false false))))))

(fn `UserConstructionScript`)